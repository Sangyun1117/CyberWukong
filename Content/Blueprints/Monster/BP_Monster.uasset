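; Base monster character, with robot dog hit assets, that chases and attacks the player and takes damage.
; SetState mirrors state to the AI Blackboard and sets walk speed; pawn sensing or damage starts a chase.
; MonsterData supplies stats, DamageReceiver drives the HP bar and death, and toggled collisions deal damage.
; Hits flash dynamic materials via timeline; skill-use and drop functions are stubs, apparently for child overrides.
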(event `SetState`
  (params (NewState :type "/Game/Blueprints/Monster/EMonsterState Enum" :default "NewEnumerator0"))
  (bind (_monsterdata_healthpower _monsterdata_attack _monsterdata_defence _monsterdata_walkspeed _monsterdata_chasespeed) (break `/Game/Blueprints/Monster/Data/OldMonsterData` (`/Game/Blueprints/Monster/Data/OldBP_MonsterData.GetMonsterData` (`self.MonsterData`))))
  ; SetState
  (if (`|EnumInequality` (`self.State_BP`) "NewEnumerator3")
    (if (`|EnumInequality` NewState (`self.State_BP`))
      (`BlackboardComponent.SetValueAsEnum` (`AIController.Blackboard` (`AIBlueprintHelperLibrary.GetAIController` self)) (`self.StateKey`) NewState)
      (bind _output_get (set `self.State_BP` NewState))
      (switch `/Game/Blueprints/Monster/EMonsterState` _output_get
        (:`NewEnumerator0`
          (set `CharacterMovementComponent.MaxWalkSpeed` _monsterdata_walkspeed (`self.CharacterMovement`)))
        (:`NewEnumerator1`
          (set `CharacterMovementComponent.MaxWalkSpeed` _monsterdata_chasespeed (`self.CharacterMovement`)))
        (:`NewEnumerator2`
          (set `CharacterMovementComponent.MaxWalkSpeed` 0.0 (`self.CharacterMovement`) :!label _label))
        (:`NewEnumerator5`
          (goto _label))
        (:`NewEnumerator6`
          (goto _label))
        (:`NewEnumerator8`
          (goto _label))
        (:`NewEnumerator3`
          (goto _label))))))

(event `self.ReceiveBeginPlay`
  (bind (_monsterdata_healthpower _monsterdata_attack _monsterdata_defence _monsterdata_walkspeed) (break `/Game/Blueprints/Monster/Data/OldMonsterData` (`/Game/Blueprints/Monster/Data/OldBP_MonsterData.GetMonsterData` (`self.MonsterData`))))
  ; BeginPlay
  (`self.OldMaterialInstanceSetting`)
  (bind _aswbp_monster_hp (cast `/Game/Blueprints/Widget/WBP_MonsterHP` (`WidgetComponent.GetUserWidgetObject` (`self.HPBar`))))
  (bind _output_get (set `self.HPBarObject` _aswbp_monster_hp))
  (`/Game/Blueprints/Widget/WBP_MonsterHP.SetMonsterInfo` _output_get (`self.Level`) (`self.MonsterName`))
  (set `/Game/Blueprints/Monster/Data/OldBP_MonsterData.MonsterName` (`self.MonsterName`) (`self.MonsterData`))
  ;; 데미지 전달 등록
  (`self.AttackCollitionSetting`)
  (for _array_element (`self.AttackCollisionArray`)
    (add `PrimitiveComponent.OnComponentBeginOverlap` _array_element (delegate `OnAnyCollisionOverlap`))
    ;; BT 이벤트 구독
    (add `DamageReceiver.OnDead` (`self.DamageReceiver`) (delegate `OnMonsterDead`))
    (add `DamageReceiver.OnHealthPowerChanged` (`self.DamageReceiver`) (delegate `OnHPChanged`))
    (set `CharacterMovementComponent.MaxWalkSpeed` _monsterdata_walkspeed (`self.CharacterMovement`))
    (`DamageReceiver.SetHp` (`self.DamageReceiver`) _monsterdata_healthpower)))

(event `OnAnyCollisionOverlap`
  (params (OverlappedComponent :type "PrimitiveComponent Object Reference") (OtherActor :type "Actor Object Reference") (OtherComp :type "PrimitiveComponent Object Reference") (OtherBodyIndex :type Integer) (bFromSweep :type Boolean) (SweepResult :type "HitResult Structure (by ref)"))
  (bind (_monsterdata_healthpower _monsterdata_attack) (break `/Game/Blueprints/Monster/Data/OldMonsterData` (`/Game/Blueprints/Monster/Data/OldBP_MonsterData.GetMonsterData` (`self.MonsterData`))))
  ; BeginPlay
  ;; 데미지 전달 등록
  (`GameplayStatics.ApplyDamage` OtherActor (* _monsterdata_attack (`self.DamageMultiplier`)) (`AIBlueprintHelperLibrary.GetAIController` self) self))

(event `OnHPChanged`
  (params (HealthPower :type "Float (single-precision)") (MaxHealthPower :type "Float (single-precision)"))
  ; BeginPlay
  ;; BT 이벤트 구독
  (`/Game/Blueprints/Widget/WBP_MonsterHP.Set HP Percent` (`self.HPBarObject`) (/ HealthPower MaxHealthPower)))

(event `TurnToTarget`
  (params (Target :type "Actor Object Reference"))
  ; 플레이어 방향으로 회전
  (`self.K2_SetActorRotation` (`KismetMathLibrary.MakeRotFromX` (`KismetMathLibrary.MakeVector` (.x (- (`self.K2_GetActorLocation` Target) (`self.K2_GetActorLocation`))) (.y (- (`self.K2_GetActorLocation` Target) (`self.K2_GetActorLocation`)))))))

(event `OnMonsterDead`
  ; BeginPlay
  ;; BT 이벤트 구독
  ;;; 죽으면 콜리전 끄기
  (`PrimitiveComponent.SetCollisionResponseToChannel` (`self.CapsuleComponent`) "ECC_GameTraceChannel3" "ECR_Ignore") ; 공중에서 죽으면 바닥을 뚫고가는 현상 막기위해 플레이어 공격만 무시
  (`PrimitiveComponent.SetCollisionEnabled` (`self.BPC_AttackCollision`) "NoCollision")
  (`self.SetState` "NewEnumerator3") ; 죽음 상태로 설정
  (`KismetSystemLibrary.Delay` 3.0)
  (`self.DropItem`)
  (`self.K2_DestroyActor`))

(event `self.PawnSensing.OnSeePawn`
  (params (Pawn :type "Pawn Object Reference"))
  ; 시야 감지
  (switch `/Game/Blueprints/Monster/EMonsterState` (`self.State_BP`)
    (:`NewEnumerator0`
      (if (not (`self.IsAttack`))
        (`BlackboardComponent.SetValueAsObject` (`AIController.Blackboard` (`AIBlueprintHelperLibrary.GetAIController` self)) (`self.TargetPlayerKey`) Pawn)
        (`self.SetState` "NewEnumerator1")))))

(event `self.ReceiveAnyDamage`
  (params (Damage :type "Float (single-precision)") (DamageType :type "DamageType Object Reference") (InstigatedBy :type "Controller Object Reference") (DamageCauser :type "Actor Object Reference"))
  (bind _returnvalue (`GameplayStatics.GetPlayerPawn` 0))
  ; 피격
  (`DamageReceiver.OnDamageReceived` (`self.DamageReceiver`) Damage)
  (`self.TurnToTarget` _returnvalue)
  (`self.OnHit`)
  (`BlackboardComponent.SetValueAsObject` (`AIController.Blackboard` (`AIBlueprintHelperLibrary.GetAIController` self)) (`self.TargetPlayerKey`) _returnvalue)
  (if (`|EnumEquality` (`self.State_BP`) "NewEnumerator0")
    (`self.SetState` "NewEnumerator1")))

(event `IsAttackToggle`
  (params (IsAttack :type Boolean))
  (set `self.IsAttack` IsAttack))

(event `OnAttackCheckBegin`
  ;[0.15 0.1324 0.006595 0.5] 공격
  (`self.AttackCollisionEnable` true))

(event `OnAttackCheckEnd`
  ;[0.15 0.1324 0.006595 0.5] 공격
  (`self.AttackCollisionEnable` false))

(event `OnHitReact`
  ; 피격
  ;; OnHitReact
  (`self.PlayAnimMontage` "/Game/Blueprints/Monster/AM_RobotDogHit.AM_RobotDogHit")
  (`GameplayStatics.PlaySound2D` "/Game/FreeSound/SC_Attack3.SC_Attack3" (`KismetMathLibrary.RandomFloatInRange` 1.0 1.0) (`KismetMathLibrary.RandomFloatInRange` 1.0 1.0) 0.0 null null)
  (`GameplayStatics.SpawnEmitterAtLocation` "/Game/FXVarietyPack/Particles/P_ky_hit2.P_ky_hit2" (`SceneComponent.K2_GetComponentLocation` (`self.CapsuleComponent`)))
  ;;; 피격 머티리얼 효과 적용
  (bind (_direction _value) (`Timeline|HitEffect` :!via `PlayFromStart`)
    (:`Update`
      (`MaterialInstanceDynamic.SetScalarParameterValue` (`self.BodyDynamicInstance`) "HitValue" _value)
      (`MaterialInstanceDynamic.SetScalarParameterValue` (`self.ArmorDynamicInstance`) "HitValue" _value))))

(fn `AttackCollisionEnable`
  (params (isEnable :type Boolean))
  (bind _bpc_attackcollision (`self.BPC_AttackCollision`))
  (if isEnable
    (`PrimitiveComponent.SetCollisionEnabled` _bpc_attackcollision "QueryOnly")
    (else
      (`PrimitiveComponent.SetCollisionEnabled` _bpc_attackcollision "NoCollision"))))

(fn `AttackCollitionSetting`
  (`KismetArrayLibrary.Array_Add` (`self.AttackCollisionArray`) (`self.BPC_AttackCollision`)))

(fn `CanUseSkill()`
  (params (Skill :type "/Game/Blueprints/Monster/EMonsterSkill Enum" :default "NewEnumerator0"))
  (returns (CanUseSkill :type Boolean))
  (return false))

(fn `DropItem`)

(fn `OldMaterialInstanceSetting`
  (bind _mesh (`self.Mesh`))
  ; 머터리얼 인스턴스 설정
  (bind _returnvalue (`PrimitiveComponent.CreateDynamicMaterialInstance` _mesh 1 "/Game/SciFi_Dog/Materials/M_SciFi_Dog_Body_Skin3.M_SciFi_Dog_Body_Skin3" "None"))
  (set `self.BodyDynamicInstance` _returnvalue)
  (bind _returnvalue_2 (`PrimitiveComponent.CreateDynamicMaterialInstance` _mesh 0 "/Game/SciFi_Dog/Materials/MI_SciFi_Dog_Armor_Skin3_Inst.MI_SciFi_Dog_Armor_Skin3_Inst" "None"))
  (set `self.ArmorDynamicInstance` _returnvalue_2))

(fn `OnHit`
  (`self.OnHitReact`))

(fn `SelectSkill`
  (bind _output_get (set `self.State_BP` "NewEnumerator2"))
  (`BlackboardComponent.SetValueAsEnum` (`AIController.Blackboard` (`AIBlueprintHelperLibrary.GetAIController` self)) (`self.StateKey`) _output_get)
  (set `CharacterMovementComponent.MaxWalkSpeed` 0.0 (`self.CharacterMovement`)))

(fn `UserConstructionScript`
  (set `self.AttackCollision` (`self.BPC_AttackCollision`)))

(fn `UseSkill`
  (params (Skill :type "/Game/Blueprints/Monster/EMonsterSkill Enum" :default "NewEnumerator0")))