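; BP_MonsterController is the AI controller for monsters, setting up their blackboard and behavior tree when it possesses a pawn.
; On possess it loads BB_Monster and writes the patrol wait time and the pawn's spawn location as the origin.
; It then casts to BP_Monster and picks BT_Monster for Dog or BT_Khaimera for Khaimera from the OldMonsterType value.
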(event `self.ReceivePossess`
  (params (PossessedPawn :type "Pawn Object Reference"))
  (`|ExecutionSequence`
    (:`then_0`
      (`self.UseBlackboard` "/Game/Blueprints/Monster/AI/BB_Monster.BB_Monster")
      (`BlackboardComponent.SetValueAsFloat` (`self.Blackboard`) (`self.PatrolWaitTimeKey`) (`self.PatrolWaitTime`))
      (`BlackboardComponent.SetValueAsVector` (`self.Blackboard`) (`self.OriginLocationKey`) (`self.K2_GetActorLocation` PossessedPawn)))
    (:`then_1`
      (bind _asbp_monster (cast `/Game/Blueprints/Monster/BP_Monster` PossessedPawn))
      (switch `/Game/Blueprints/Monster/EMonsterType` (`/Game/Blueprints/Monster/BP_Monster.OldMonsterType` _asbp_monster)
        (:`NewEnumerator0`
          (`self.RunBehaviorTree` "/Game/Blueprints/Monster/AI/BT_Monster.BT_Monster"))
        (:`NewEnumerator1`
          (`self.RunBehaviorTree` "/Game/Blueprints/Monster/AI/BT_Khaimera.BT_Khaimera"))))))

(fn `UserConstructionScript`)