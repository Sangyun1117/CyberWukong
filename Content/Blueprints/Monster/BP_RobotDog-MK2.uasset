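; BP_RobotDog-MK2 is a robot dog monster Blueprint that defines how it reacts to being hit.
; OnHit fires a hit-react event that plays a montage, a 2D sound and an impact emitter at the capsule.
; A timeline then drives a HitValue scalar on body and armor dynamic materials for a hit effect.
; OldMaterialInstanceSetting creates those material instances, while the construction script only calls its parent.
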(event `MyOnHitReact`
  (`self.PlayAnimMontage` "/Game/Blueprints/Monster/AM_RobotDogHit.AM_RobotDogHit")
  (`GameplayStatics.PlaySound2D` "/Game/FreeSound/SC_Attack3.SC_Attack3" (`KismetMathLibrary.RandomFloatInRange` 1.0 1.0) (`KismetMathLibrary.RandomFloatInRange` 1.0 1.0) 0.0 null null)
  (`GameplayStatics.SpawnEmitterAtLocation` "/Game/FXVarietyPack/Particles/P_ky_hit2.P_ky_hit2" (`SceneComponent.K2_GetComponentLocation` (`self.CapsuleComponent`)))
  ; 피격 머티리얼 효과 적용
  (bind (_direction _value) (`Timeline|타임라인` :!via `PlayFromStart`)
    (:`Update`
      (`MaterialInstanceDynamic.SetScalarParameterValue` (`self.BodyDynamicInstance`) "HitValue" _value)
      (`MaterialInstanceDynamic.SetScalarParameterValue` (`self.ArmorDynamicInstance`) "HitValue" _value))))

(fn `OldMaterialInstanceSetting`
  (bind _mesh (`self.Mesh`))
  ; 머터리얼 인스턴스 설정
  (bind _returnvalue (`PrimitiveComponent.CreateDynamicMaterialInstance` _mesh 1 "/Game/SciFi_Dog/Materials/M_SciFi_Dog_Body_Skin1.M_SciFi_Dog_Body_Skin1" "None"))
  (set `self.BodyDynamicInstance` _returnvalue)
  (bind _returnvalue_2 (`PrimitiveComponent.CreateDynamicMaterialInstance` _mesh 0 "/Game/SciFi_Dog/Materials/MI_SciFi_Dog_Armor_Skin1_Inst.MI_SciFi_Dog_Armor_Skin1_Inst" "None"))
  (set `self.ArmorDynamicInstance` _returnvalue_2))

(fn `OnHit`
  (`self.MyOnHitReact`))

(fn `UserConstructionScript`
  (`parent.UserConstructionScript`))