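; BP_Wukong is the Wukong player character Blueprint, handling HUD setup, combat montages and damage feedback.
; BeginPlay creates the game screen and caches its HUD, minimap and interaction text, while Tick updates decoration transparency, minimap material parameters and slam-push wall checks.
; PlayMontage drives combo attacks, rolls and slam pushes; damage goes to DamageReceiver with sound and particles.
; A DoN reset on landing gates upward launches, and P/R keys toggle slow motion.
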(event `UpdateMinimapInfo`
  ; 미니맵
  (`KismetMaterialLibrary.SetVectorParameterValue` "/Game/Blueprints/Widget/MiniMap/MP_Minimap.MP_Minimap" "PlayerLocation" (`KismetMathLibrary.Conv_VectorToLinearColor` (`self.K2_GetActorLocation`)))
  (`KismetMaterialLibrary.SetScalarParameterValue` "/Game/Blueprints/Widget/MiniMap/MP_Minimap.MP_Minimap" "Player Yaw" (/ (+ (.yaw (`self.K2_GetActorRotation`)) 180.0) 360.0)))

(event `self.ReceiveTick`
  (params (DeltaSeconds :type "Float (single-precision)"))
  ; Tick
  (`self.TransparencyDecorations`)
  (`self.UpdateMinimapInfo`)
  (`self.SlamPushWallCheck`))

(event `self.ReceiveBeginPlay`
  ; BeginPlay
  ;; 플레이어HUD 설정
  (bind _returnvalue (`|CreateWidget` "/Game/Blueprints/Widget/WBP_GameScreen.WBP_GameScreen_C"))
  (`UserWidget.AddToViewport` _returnvalue 0)
  (bind _output_get (set `self.PlayerHUD` (`/Game/Blueprints/Widget/WBP_GameScreen.WBP_PlayerHUD` _returnvalue)))
  (`/Game/Blueprints/Widget/WBP_PlayerHUD.SetHP` _output_get (`self.CurrentHp`) (`self.MaxHp`))
  (set `self.Minimap` (`/Game/Blueprints/Widget/WBP_GameScreen.WBP_Minimap` _returnvalue))
  (set `self.InteractionText` (`/Game/Blueprints/Widget/WBP_GameScreen.WBP_InteractionText` _returnvalue))
  (`/Game/Blueprints/Widget/WBP_PlayerHUD.SetEP` _output_get (`self.CurrentEp`) (`self.MaxEp`)))

(event `self.PlayMontage`
  (params (Effect :type "EEffectType Enum" :default "Attack"))
  ; 애니메이션 호출
  (switch `EEffectType` Effect
    (:`Attack`
      (switch `name` (`self.NextCombo`)
        (:`Default`
          (`AnimInstance.Montage_JumpToSection` (`SkeletalMeshComponent.GetAnimInstance` (`self.Mesh`)) (`self.NextCombo`) "/Game/Blueprints/Character/AM_WukongAttack.AM_WukongAttack"))
        (:`Attack1`
          (`self.PlayAnimMontage` "/Game/Blueprints/Character/AM_WukongAttack.AM_WukongAttack" 1.0 "Attack1"))))
    (:`Roll`
      (`self.PlayAnimMontage` "/Game/Blueprints/Character/AM_Quick_Roll_To_Run.AM_Quick_Roll_To_Run"))
    (:`SlamPush`
      (`self.PlayAnimMontage` "/Game/Blueprints/Character/AM_WukongSlam.AM_WukongSlam" 1.0 "SlamPush"))
    (:`SlamPushStop`
      (`self.StopAnimMontage` "/Game/Blueprints/Character/AM_WukongSlam.AM_WukongSlam")
      (bind _asabp_wukong (cast `/Game/Blueprints/Character/ABP_Wukong` (`SkeletalMeshComponent.GetAnimInstance` (`self.Mesh`))))
      (`/Game/Blueprints/Character/ABP_Wukong.SlamExit` _asabp_wukong))))

(event `MoveEnable`
  (params (CanMove :type Boolean))
  ; 플레이어 이동
  (set `self.bCanMove` CanMove))

(event `self.OnLanded`
  (params (Hit :type "HitResult Structure (by ref)"))
  ; 플레이어 이동
  (`/Engine/EditorBlueprintResources/StandardMacros.Do N` 2 :!via `Reset`
    (:`Exit`
      (`self.LaunchCharacter` (0.0 0.0 400.0) false true))))

(event `self.ReceiveAnyDamage`
  (params (Damage :type "Float (single-precision)") (DamageType :type "DamageType Object Reference") (InstigatedBy :type "Controller Object Reference") (DamageCauser :type "Actor Object Reference"))
  ; 피격
  (`DamageReceiver.OnDamageReceived` (`self.DamageReceiver`) Damage)
  (`GameplayStatics.PlaySound2D` "/Game/FreeSound/SC_Attack3.SC_Attack3" (`KismetMathLibrary.RandomFloatInRange` 1.0 1.0) (`KismetMathLibrary.RandomFloatInRange` 1.0 1.0) 0.0 null null)
  (`GameplayStatics.SpawnEmitterAtLocation` "/Game/FXVarietyPack/Particles/P_ky_hit1.P_ky_hit1" (`SceneComponent.K2_GetComponentLocation` (`self.CapsuleComponent`)) (struct) (0.5 0.5 0.5)))

(event `Key|P`
  (params (Key :type "Key Structure"))
  (:`Pressed`
    (`GameplayStatics.SetGlobalTimeDilation` 0.5)))

(event `Key|R`
  (params (Key :type "Key Structure"))
  (:`Pressed`
    (`GameplayStatics.SetGlobalTimeDilation` 1.0)))

(fn `UserConstructionScript`
  (set `self.AttackCollision` (`self.BPC_AttackCollision`))
  (set `self.SlamPushCollision` (`self.BPC_SlamPushCollision`))
  (set `self.SlamDownCollision` (`self.BPC_SlamDownCollision`)))