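; BP_TreasureChest is a treasure chest that ends the game when BP_Wukong enters its overlap box while holding a key.
; With the key, it rotates the lid open, shows the WBP_GameClear widget and starts a short timer that loads IntroMap.
; Without the key, it tells the player through Wukong's interaction message that there is no key.
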(event `self.Box.OnComponentBeginOverlap`
  (params (OverlappedComponent :type "PrimitiveComponent Object Reference") (OtherActor :type "Actor Object Reference") (OtherComp :type "PrimitiveComponent Object Reference") (OtherBodyIndex :type Integer) (bFromSweep :type Boolean) (SweepResult :type "HitResult Structure (by ref)"))
  (bind _asbp_wukong (cast `/Game/Blueprints/Character/BP_Wukong` OtherActor))
  (if (`Wukong.bIsKey` _asbp_wukong)
    (`SceneComponent.K2_SetRelativeRotation` (`self.ChestLid`) (struct :`Roll` -90.0) false false)
    (bind _returnvalue (`|CreateWidget` "/Game/Blueprints/Widget/WBP_GameClear.WBP_GameClear_C"))
    (`UserWidget.AddToViewport` _returnvalue 0)
    (`KismetSystemLibrary.K2_SetTimerDelegate` (delegate `BackHome`) 3.0)
    (else
      (`Wukong.ShowInteraction` _asbp_wukong "열쇠가 없습니다."))))

(event `BackHome`
  (`GameplayStatics.OpenLevel` "IntroMap"))

(fn `UserConstructionScript`)